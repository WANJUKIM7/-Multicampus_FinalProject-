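; Table lamp prop for the Victorian mansion set, with a power cord that can be shaped along a spline.
; The construction script adds a spline mesh segment between each pair of neighboring spline points, matching their positions and tangents to form the cord.
; It then places a plug static mesh at the first point, rotated along that point's tangent.
; The event graph holds no runtime logic.
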(fn `UserConstructionScript`
  (bind _spline (`self.Spline`))
  (bind _spline_2 (`self.Spline`))
  (bind (_location _tangent) (`SplineComponent.GetLocationAndTangentAtSplinePoint` _spline 0 "Local"))
  (for _index (range (+ (- (`SplineComponent.GetNumberOfSplinePoints` _spline) 2) 1))
    ;[1 1 1] Cord Spline
    (bind _returnvalue (`AddComponent|NODE_AddSplineMeshComponent-6`))
    (`SceneComponent.K2_AttachToComponent` _returnvalue (`self.Spline Mesh`) "None" "KeepRelative" "KeepRelative" "KeepRelative" true)
    (bind (_location_2 _tangent_2) (`SplineComponent.GetLocationAndTangentAtSplinePoint` _spline_2 _index "Local"))
    (bind (_location_3 _tangent_3) (`SplineComponent.GetLocationAndTangentAtSplinePoint` _spline_2 (+ _index 1) "Local"))
    (`SplineMeshComponent.SetStartAndEnd` _returnvalue _location_2 _tangent_2 _location_3 _tangent_3 true))
  ;[1 1 1] Plug Static Mesh
  (bind _returnvalue_2 (`AddComponent|NODE_AddStaticMeshComponent-0`))
  (`SceneComponent.K2_SetRelativeLocation` _returnvalue_2 _location false false)
  (`SceneComponent.K2_SetRelativeRotation` _returnvalue_2 (`KismetMathLibrary.Conv_VectorToRotator` _tangent) false false))