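; Construction-only Blueprint that places repeated static meshes along a spline, named as roof cresting for the Victorian mansion asset set.
; The construction script divides the spline length by Spacing and adds a Static Mesh component at each step, including the start.
; Each component uses manual attachment and takes the world-space location and rotation at that distance, at unit scale, so pieces are placed rigidly rather than deformed as spline meshes.
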(fn `UserConstructionScript`
  (bind _spacing (`self.Spacing`))
  (for _index (range (+ (`.ReturnValue` (`KismetMathLibrary.FMod` (`SplineComponent.GetSplineLength` (`self.Spline`)) _spacing)) 1))
    (bind _returnvalue (* _index _spacing))
    (bind _returnvalue_2 (`AddComponent|NODE_AddStaticMeshComponent-0` :`bManualAttachment` true :`RelativeTransform` (`KismetMathLibrary.MakeTransform` (`SplineComponent.GetLocationAtDistanceAlongSpline` (`self.Spline`) _returnvalue "World") (`SplineComponent.GetRotationAtDistanceAlongSpline` (`self.Spline`) _returnvalue "World"))))
    (`StaticMeshComponent.SetStaticMesh` _returnvalue_2 (`self.Static Mesh`))))