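; Breakable platform that loses durability when overlapped after the game has started and destroys itself at zero.
; Three box collisions share one overlap path, gated by a flag so only one hit registers at a time.
; At one durability left, it creates a dynamic material with zero brightness and re-arms after a short delay.
; At zero, it calls ShakeAndDestroy, brightens, and animates opacity on a timeline before destroying the actor.
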(event `SetGameStarted`
  ;[1 1 1] 게임 시작 여부
  (set `self.IsGameStarted` true))

(event `self.BoxCollision.OnComponentBeginOverlap`
  (params (OverlappedComponent :type "PrimitiveComponent Object Reference") (OtherActor :type "Actor Object Reference") (OtherComp :type "PrimitiveComponent Object Reference") (OtherBodyIndex :type Integer) (bFromSweep :type Boolean) (SweepResult :type "HitResult Structure (by ref)"))
  ;[1 1 1] 발판이랑 캐릭터 오버랩시
  (if (`self.IsGameStarted`) :!label _label
    (if (not (`self.IsBeingOverlapped`))
      (set `self.IsBeingOverlapped` true)
      (bind _output_get (set `self.Durability` (- (`self.Durability`) 1)))
      (switch `int` _output_get
        (:`0`
          ;;[1 1 1] 내구도 0일시 깨지기
          (`self.ChangeMaterialAndDestroy`))
        (:`1`
          (`|ExecutionSequence`
            (:`then_0`
              ;;[1 1 1] 머티리얼 바꾸기
              (bind _returnvalue (`PrimitiveComponent.CreateDynamicMaterialInstance` (`self.Platform`) 0 "/Game/Programming/Materials/MM_Bright.MM_Bright" "None"))
              (bind _output_get_2 (set `self.DynamicMaterialInstance` _returnvalue))
              (`MaterialInstanceDynamic.SetScalarParameterValue` _output_get_2 "Bright" 0.0)
              (`KismetSystemLibrary.Delay` 0.5)
              (set `self.IsBeingOverlapped` false :!label _label_2))))))))

(event `self.BoxCollision1.OnComponentBeginOverlap`
  (params (OverlappedComponent :type "PrimitiveComponent Object Reference") (OtherActor :type "Actor Object Reference") (OtherComp :type "PrimitiveComponent Object Reference") (OtherBodyIndex :type Integer) (bFromSweep :type Boolean) (SweepResult :type "HitResult Structure (by ref)"))
  ;[1 1 1] 발판이랑 캐릭터 오버랩시
  (goto _label))

(event `self.BoxCollision2.OnComponentBeginOverlap`
  (params (OverlappedComponent :type "PrimitiveComponent Object Reference") (OtherActor :type "Actor Object Reference") (OtherComp :type "PrimitiveComponent Object Reference") (OtherBodyIndex :type Integer) (bFromSweep :type Boolean) (SweepResult :type "HitResult Structure (by ref)"))
  ;[1 1 1] 발판이랑 캐릭터 오버랩시
  (goto _label))

(event `ChangeMaterialAndDestroy`
  ;[1 1 1] 발판이랑 캐릭터 오버랩시
  ;;[1 1 1] 머티리얼 변하면서 파괴
  (`self.ShakeAndDestroy`)
  (set `self.IsTimePassed` false)
  (`MaterialInstanceDynamic.SetScalarParameterValue` (`self.DynamicMaterialInstance`) "Bright" 10.0)
  (bind (_direction _value) (`Timeline|타임라인`)
    (:`Update`
      (`MaterialInstanceDynamic.SetScalarParameterValue` (`self.DynamicMaterialInstance`) "Opacity" _value))
    (:`Finished`
      (`self.K2_DestroyActor`)
      (goto _label_2))))

(fn `UserConstructionScript`)