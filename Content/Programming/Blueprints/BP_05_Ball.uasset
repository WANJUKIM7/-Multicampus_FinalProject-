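; BP_05_Ball is an actor attached to a BP_Player that knocks other players away on overlap.
; When the overlapped actor's attach parent is also a BP_Player, it spawns a hit emitter at the midpoint between both players.
; It then launches that player along X and Y, away from its own, using the unnormalized offset times HitPower, and prints debug text.
; The component hit event is empty.
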(event `self.Ball.OnComponentHit`
  (params (HitComponent :type "PrimitiveComponent Object Reference") (OtherActor :type "Actor Object Reference") (OtherComp :type "PrimitiveComponent Object Reference") (NormalImpulse :type "Vector Structure") (Hit :type "HitResult Structure (by ref)"))
  ;[1 1 1] HIt 불가능 판정
)

(event `self.Ball.OnComponentBeginOverlap`
  (params (OverlappedComponent :type "PrimitiveComponent Object Reference") (OtherActor :type "Actor Object Reference") (OtherComp :type "PrimitiveComponent Object Reference") (OtherBodyIndex :type Integer) (bFromSweep :type Boolean) (SweepResult :type "HitResult Structure (by ref)"))
  (bind _hitpower (`self.HitPower`))
  (bind _returnvalue (`self.K2_GetActorLocation` (cast `/Game/Programming/Blueprints/BP_Player` (`self.GetAttachParentActor`) :!pure true)))
  ;[1 1 1] 플레이어들 위치 가져오기
  (bind _asbp_player (cast `/Game/Programming/Blueprints/BP_Player` (`self.GetAttachParentActor` OtherActor)))
  (`|ExecutionSequence`
    (:`then_0`
      (bind _returnvalue_2 (`self.K2_GetActorLocation` _asbp_player))
      ;[1 1 1] 효과 생성
      (bind _output_get (set `self.HitLocation` (/ (+ _returnvalue_2 _returnvalue) (2.0 2.0 2.0))))
      (`GameplayStatics.SpawnEmitterAtLocation` "/Game/contents/VFX/Realistic_Starter_VFX_Pack_Vol2/Particles/Explosion/VFX_04_GetHit.VFX_04_GetHit" _output_get))
    (:`then_1`
      ;[1 1 1] 캐릭터 밀치기
      (bind _output_get_2 (set `self.HitVector` (- _returnvalue_2 _returnvalue)))
      (`Character.LaunchCharacter` _asbp_player (`KismetMathLibrary.MakeVector` (* (.x _output_get_2) _hitpower) (* (.y _output_get_2) _hitpower)) true false)
      (`KismetSystemLibrary.PrintText` "Hello"))))

(fn `UserConstructionScript`)