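; BP_05_InclinePlatform is a platform that tilts under physics simulation, with its incline kept within a set limit.
; BeginPlay turns on physics for the InclinePlatform component, and a SimulateOn event enables it again.
; Every Tick clamps relative roll and pitch to plus or minus InclineValue and forces yaw to zero.
; An EnableInput call is left unconnected and never runs.
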(event `self.ReceiveBeginPlay`
  ;[1 1 1] 시뮬레이트 작동 끄기
  (`PrimitiveComponent.SetSimulatePhysics` (`self.InclinePlatform`) true))

(event `self.ReceiveTick`
  (params (DeltaSeconds :type "Float (single-precision)"))
  (bind _inclineplatform (`self.InclinePlatform`))
  (bind _inclinevalue (`self.InclineValue`))
  (bind _returnvalue (* _inclinevalue -1.0))
  (bind (_relativerotation_roll _relativerotation_pitch) (`KismetMathLibrary.BreakRotator` (`SceneComponent.RelativeRotation` _inclineplatform)))
  ;[1 1 1] 기울기 조절
  (`SceneComponent.K2_SetRelativeRotation` _inclineplatform (`KismetMathLibrary.MakeRotator` (`KismetMathLibrary.FClamp` _relativerotation_roll _returnvalue _inclinevalue) (`KismetMathLibrary.FClamp` _relativerotation_pitch _returnvalue _inclinevalue)) false false))

(event `SimulateOn`
  ;[1 1 1] 시뮬레이트 작동 켜기
  (`PrimitiveComponent.SetSimulatePhysics` (`self.InclinePlatform`) true))

(fn `UserConstructionScript`)