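; BP_08_CannonBall is a cannonball that grows in size and rolls along a given direction.
; On BeginPlay a timeline scales the CannonBall component up to CannonBallScale, then prints "Complete".
; Every Tick adds a velocity-change impulse along ForwardVector multiplied by CannonBallScale, so acceleration depends on frame rate.
; The SetForwardVector event stores the travel direction passed in by its caller.
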(event `self.ReceiveBeginPlay`
  ;[1 1 1] 크기 커지기
  (bind (_direction _scale) (`Timeline|타임라인`)
    (:`Update`
      (`SceneComponent.SetRelativeScale3D` (`self.CannonBall`) (`KismetMathLibrary.Conv_DoubleToVector` (* _scale (`self.CannonBallScale`)))))
    (:`Finished`
      (`KismetSystemLibrary.PrintText` "Complete"))))

(event `self.ReceiveTick`
  (params (DeltaSeconds :type "Float (single-precision)"))
  ;[1 1 1] 공 굴러가게
  (`PrimitiveComponent.AddImpulse` (`self.CannonBall`) (* (`self.ForwardVector`) (`self.CannonBallScale`)) "None" true))

(event `SetForwardVector`
  (params (ForwardVector :type "Vector Structure"))
  ;[1 1 1] 앞벡터 세팅
  (set `self.ForwardVector` ForwardVector))

(fn `UserConstructionScript`)