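; BP_06_Tail is a tail actor that builds a trail of cylinder spline meshes along its Tail spline.
; SpawnSplineMesh appends a world-space point, spans a new overlap-enabled segment from the previous point and records it with its creation time.
; Tick destroys the oldest segment once its age reaches TimeLifeSpan, which SetSplineMeshLifeSpan extends, leaving spline points in place.
; BeginPlay disables Tick, and nothing here re-enables it.
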(event `self.ReceiveBeginPlay`
  ;[1 1 1] BeginPlay
  (`self.SetActorTickEnabled` false))

(event `SetSplineMeshLifeSpan`
  ;[1 1 1] 꼬리 수명 최신화
  (set `self.TimeLifeSpan` (+ (`self.TimeLifeSpan`) 0.5)))

(event `self.ReceiveTick`
  (params (DeltaSeconds :type "Float (single-precision)"))
  (bind (_output_splinemesh _output_time) (break `/Game/Programming/Structs/F_SplineMesh` (`|GetArrayItem` (`self.F_SplineMesh`))))
  ;[1 1 1] SplineMesh 자동 파괴
  (`/Engine/EditorBlueprintResources/StandardMacros.IsValid` _output_splinemesh
    (:`Is Valid`
      (if (>= (- (`self.GetGameTimeSinceCreation`) _output_time) (`self.TimeLifeSpan`))
        (`ActorComponent.K2_DestroyComponent` _output_splinemesh)
        (`KismetArrayLibrary.Array_Remove` (`self.F_SplineMesh`))
        (else
          (`KismetSystemLibrary.PrintText` "No SplineMesh"))))))

(event `SpawnSplineMesh`
  (params (Position :type "Vector Structure"))
  (bind _splinepointsnumber (`self.SplinePointsNumber`))
  (bind _tail (`self.Tail`))
  (bind _tail_2 (`self.Tail`))
  ;[1 1 1] spline point, splinemesh
  (`SplineComponent.AddSplinePoint` _tail Position "World" true)
  (set `self.SplinePointsNumber` (`SplineComponent.GetNumberOfSplinePoints` _tail))
  (`|ExecutionSequence`
    (:`then_0`
      (bind _returnvalue (`AddComponent|NODE_AddSplineMeshComponent-0` :`self` self :`bManualAttachment` true))
      (bind _output_get (set `self.SplineMesh` (make `/Game/Programming/Structs/F_SplineMesh` _returnvalue (`self.GetGameTimeSinceCreation`))))
      (`KismetArrayLibrary.Array_Add` (`self.F_SplineMesh`) _output_get)
      (`self.SetActorEnableCollision` true)
      (`PrimitiveComponent.SetCollisionEnabled` _returnvalue "QueryAndPhysics")
      (`PrimitiveComponent.SetCollisionObjectType` _returnvalue "ECC_WorldDynamic")
      (`PrimitiveComponent.SetCollisionResponseToAllChannels` _returnvalue "ECR_Overlap")
      (set `PrimitiveComponent.bGenerateOverlapEvents` true _returnvalue))
    (:`then_1`
      (`StaticMeshComponent.SetStaticMesh` _returnvalue "/Game/LevelDesign/LevelPrototyping/Meshes/SM_Cylinder.SM_Cylinder")
      (`PrimitiveComponent.SetMaterial` _returnvalue 0 "/Game/StarterContent/Props/Materials/M_Lamp.M_Lamp")
      (`SplineMeshComponent.SetStartScale` _returnvalue (0.2 0.2) true)
      (`SplineMeshComponent.SetEndScale` _returnvalue (0.2 0.2) true)
      (`SplineMeshComponent.SetForwardAxis` _returnvalue "X" true)
      (`SplineMeshComponent.SetStartAndEnd` _returnvalue (`SplineComponent.GetLocationAtSplinePoint` _tail_2 (- _splinepointsnumber 2) "World") (0.0 0.0 0.0) (`SplineComponent.GetLocationAtSplinePoint` _tail_2 (- _splinepointsnumber 1) "World") (0.0 0.0 0.0) true))))

(fn `UserConstructionScript`)