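; BP_08_Cannon is a cannon actor that repeatedly fires BP_08_CannonBall actors on a looping timer started at BeginPlay.
; Each ball spawns at the middle arrow's transform and receives that arrow's forward vector as its direction.
; When RandomWay is enabled, it also gets a scaled physics impulse along a random blend of the left and right arrows' forward vectors, spreading the shots.
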(event `self.ReceiveBeginPlay`
  ;[1 1 1] 대포알 생성
  (`KismetSystemLibrary.K2_SetTimerDelegate` (delegate `SpawnCannonBall`) (`self.TimeLoopSpawnCannonBall`) true))

(event `SpawnCannonBall`
  ;[1 1 1] 대포알 생성
  (bind _returnvalue (`|SpawnActorFromClass` "/Game/Programming/Blueprints/BP_08_CannonBall.BP_08_CannonBall_C" (`SceneComponent.K2_GetComponentToWorld` (`self.ArrowMiddle`)) "Undefined" "MultiplyWithRoot" null null))
  (`/Game/Programming/Blueprints/BP_08_CannonBall.SetForwardVector` _returnvalue (`SceneComponent.GetForwardVector` (`self.ArrowMiddle`)))
  (if (`self.bRandomWay`)
    (`PrimitiveComponent.AddImpulse` (`FP08CannonBall.CannonBall` _returnvalue) (* (`KismetMathLibrary.VLerp` (`SceneComponent.GetForwardVector` (`self.ArrowLeft`)) (`SceneComponent.GetForwardVector` (`self.ArrowRight`)) (`KismetMathLibrary.RandomFloat`)) (`self.RandomWayValue`)) "None" false)))

(fn `UserConstructionScript`)